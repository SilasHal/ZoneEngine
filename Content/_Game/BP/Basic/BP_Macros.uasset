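; BP_Macros is a basic Blueprint that demonstrates a macro setting two variables.
; The Set Value macro takes one input, stores it in Current, and stores that input plus a fixed offset in Counter.
; BeginPlay calls the macro with zero, then prints both variables as strings.
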(event `self.ReceiveBeginPlay`
  (`self.Set Value` 0
    (:`out`
      (`KismetSystemLibrary.PrintString` (`KismetStringLibrary.Conv_IntToString` (`self.Current`)))
      (`KismetSystemLibrary.PrintString` (`KismetStringLibrary.Conv_IntToString` (`self.Counter`))))))

(fn `UserConstructionScript`)