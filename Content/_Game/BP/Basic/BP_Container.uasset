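; BP_Container is an Actor that exercises Blueprint container types (Map, Set, Array) through debug prints.
; BeginPlay prints the Name of each struct value in NameMap, each time also printing the HP stored under key "s", or "Hello" if absent.
; EndPlay clears NameArray.
; Unconnected graphs hold further experiments with Set add and lookup, Map key iteration and random Array picks in a while loop.
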(event `self.ReceiveBeginPlay`
  (bind _namemap (`self.NameMap`))
  (bind (_value _returnvalue) (`BlueprintMapLibrary.Map_Find` _namemap "s"))
  (bind _values (`BlueprintMapLibrary.Map_Values` _namemap))
  (for _array_element _values
    (`KismetSystemLibrary.PrintString` (break `/Game/_Game/Structures/S_PlayerStruct` _array_element))
    (if _returnvalue
      (`KismetSystemLibrary.PrintString` (`KismetStringLibrary.Conv_DoubleToString` (`.HP_6_2E57FE964C4A51373B024FB05C08C148` (break `/Game/_Game/Structures/S_PlayerStruct` _value))))
      (else
        (`KismetSystemLibrary.PrintString` "Hello")))))

(event `self.ReceiveEndPlay`
  (params (EndPlayReason :type "EEndPlayReason Enum" :default "Destroyed"))
  (`KismetArrayLibrary.Array_Clear` (`self.NameArray`)))

(fn `UserConstructionScript`)