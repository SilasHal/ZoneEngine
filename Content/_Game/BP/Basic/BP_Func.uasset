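; BP_Func is a small Blueprint that demonstrates a custom function with a branch and return value.
; On BeginPlay it passes First to NewValue, stores the result in Second and prints it.
; NewValue adds ten to inputs below ten, using a local copy, and returns other values unchanged.
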(event `self.ReceiveBeginPlay`
  (bind _returnvalue (`self.NewValue` (`self.First`)))
  (bind _output_get (set `self.Second` _returnvalue))
  (`KismetSystemLibrary.PrintString` (`KismetStringLibrary.Conv_IntToString` _output_get)))

(fn `NewValue`
  (params (Val :type Integer))
  (returns (ReturnValue :type Integer))
  (locals (Var :type Integer))
  (if (< Val 10)
    (bind _output_get (set `local.Var` Val))
    (return (+ _output_get 10))
    (else
      (return Val))))

(fn `UserConstructionScript`)